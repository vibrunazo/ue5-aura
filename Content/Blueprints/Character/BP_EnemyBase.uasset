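; BP_EnemyBase is the base enemy character Blueprint, handling spawn, death and facing visuals.
; On BeginPlay it binds its death event and scales the mesh through a spawn timeline; on death it applies the GE_Dead gameplay effect to itself.
; Separate timelines drive the Dissolve parameter on supplied dynamic materials, one of them for the weapon.
; A Motion Warping event updates the FacingTarget location.
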(event Custom|OnDied_Event
  (params (DyingCharacter :type Aura%20Character%20Base%20Object%20Reference))
  (GameplayEffects|ApplyGameplayEffectToSelf :self (Ability|GetAbilitySystemComponent 0) :GameplayEffectClass "/Game/Blueprints/AbilitySystem/Enemy/Effects/GE_Dead.GE_Dead_C"))

(event EventBeginPlay
  (|CallParentFunction)
  (EventDispatchers|AssignOnDied (delegate Custom|OnDied_Event))
  (bind _scalecurve (Timeline|SpawnTweening Play)
    (:Update
      (Transformation|SetRelativeScale3D (Variables|Character|GetMesh) (Math|Vector|MakeVector _scalecurve _scalecurve _scalecurve)))))

(event EventStartDissolveTimeline
  (params (MaterialInstanceDynamic :type Material%20Instance%20Dynamic%20Object%20Reference))
  (bind _dissolvetrack (Timeline|DissolveTimeline Play)
    (:Update
      (Rendering|Material|SetScalarParameterValue MaterialInstanceDynamic "Dissolve" _dissolvetrack :!class /Script/Engine.MaterialInstanceDynamic))))

(event EventStartWeaponDissolveTimeline
  (params (MaterialInstanceDynamic :type Material%20Instance%20Dynamic%20Object%20Reference))
  (bind _dissolvetrack (Timeline|Timeline Play)
    (:Update
      (Rendering|Material|SetScalarParameterValue MaterialInstanceDynamic "Dissolve" _dissolvetrack :!class /Script/Engine.MaterialInstanceDynamic))))

(event EventSetMotionWarpTarget
  (params (TargetLocation :type Vector%20%28by%20ref%29 :default "0, 0, 0"))
  (Class|MotionWarpingComponent|AddorUpdateWarpTargetfromLocation (Variables|Default|GetMotionWarping) "FacingTarget" TargetLocation))

(fn ConstructionScript)
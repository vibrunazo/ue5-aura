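; Enemy gameplay ability that performs a ranged attack, firing a projectile at the avatar's combat target.
; It picks a random attack montage from the avatar, plays it, and sets the motion warp target to the combat target's location.
; A gameplay event matching the montage's tag triggers the projectile cast from the montage's socket, aimed at the target with a Z offset.
; The ability ends when the montage completes, is interrupted or is cancelled.
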(event Ability|EventActivateAbility
  (bind _returnvalue (Ability|GetAvatarActorfromActorInfo))
  (bind _returnvalue_2 (Class|CombatInterface|GetAttackMontages(Message) (Ability|GetAvatarActorfromActorInfo)))
  (bind _output_get (Variables|Default|SetCurrentTaggerMontage (.OutItem (Utilities|Array|Random _returnvalue_2))))
  (Variables|Default|SetMontage%20Tag (.MontageTag (Utilities|Struct|BreakTaggedMontage _output_get)))
  (Variables|Default|SetSocket%20Tag (.SocketTag (Utilities|Struct|BreakTaggedMontage _output_get)))
  (|PlayMontageandWaitProxy "None" (.Montage (Utilities|Struct|BreakTaggedMontage _output_get)) 1.0 "None" false 1.0 0.0 false
    (:then
      (bind _returnvalue_3 (Class|EnemyInterface|GetCombatTarget(Message) _returnvalue))
      (Class|CombatInterface|SetMotionWarpTarget(Message) _returnvalue (Transformation|GetActorLocation _returnvalue_3))
      (Ability|Tasks|WaitGameplayEvent (Variables|Default|GetMontage%20Tag) 0
        (:EventReceived
          (Class|AuraProjectileSpell|CastProjectile (Math|Vector|MakeVector (.X (Math|Vector|BreakVector (Transformation|GetActorLocation _returnvalue_3))) (.Y (Math|Vector|BreakVector (Transformation|GetActorLocation _returnvalue_3))) (+ (.Z (Math|Vector|BreakVector (Transformation|GetActorLocation _returnvalue_3))) (Variables|Default|GetZ-Offset))) (Variables|Default|GetSocket%20Tag)))))
    (:OnCompleted
      (Ability|EndAbility :!label _label))
    (:OnInterrupted
      (goto _label))
    (:OnCancelled
      (goto _label))))
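; GA_HitReact is the enemy gameplay ability that plays a hit reaction.
; On activation it applies GE_HitReact to the owner and plays the montage supplied by the avatar's CombatInterface.
; It also sets the aggro key in the avatar's blackboard to true.
; When the montage completes, blends out, is interrupted or is cancelled, it removes the effect by its stored handle and ends the ability.
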(event Ability|EventActivateAbility
  (bind _returnvalue (Ability|GetAvatarActorfromActorInfo))
  (bind _returnvalue_2 (Ability|ApplyGameplayEffectToOwner "/Game/Blueprints/AbilitySystem/Enemy/Effects/GE_HitReact.GE_HitReact_C"))
  (Variables|Default|SetActiveEffect _returnvalue_2)
  (Utilities|FlowControl|Sequence
    (:then_0
      (bind _ascombat_interface (Utilities|Casting|CastToCombatInterface _returnvalue))
      (bind _returnvalue_3 (Class|CombatInterface|GetHitReactMontage _ascombat_interface))
      (|PlayMontageandWaitProxy "None" _returnvalue_3 1.0 "None" true 1.0 0.0 false
        (:OnCompleted
          _)
        (:OnBlendOut
          _)
        (:OnInterrupted
          _)
        (:OnCancelled
          _))
      (Ability|RemoveGameplayEffectFromOwnerWithHandle (Variables|Default|GetActiveEffect))
      (Ability|EndAbility))
    (:then_1
      (Utilities|IsValid _returnvalue
        (:Is%20Valid
          (AI|Components|Blackboard|SetValueasBool (AI|GetBlackboard _returnvalue) (Variables|Default|GetAggroKey%20Name) true))))))

(event Ability|EventOnEndAbility
  (params (bWasCancelled :type Boolean)))
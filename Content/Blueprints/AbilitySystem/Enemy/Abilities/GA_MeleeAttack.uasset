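; Enemy melee attack gameplay ability that plays a random tagged attack montage and motion-warps the avatar toward its combat target.
; On the montage's tagged gameplay event, it finds live players within a small sphere at the tagged combat socket and damages enemy-team hits.
; Any hit fires one MeleeImpact gameplay cue at the socket, not yet one per target.
; The ability ends when the montage completes, is interrupted or is cancelled.
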(event Ability|EventActivateAbility
  (bind _returnvalue (Ability|GetAvatarActorfromActorInfo))
  (bind _returnvalue_2 (Ability|GetAvatarActorfromActorInfo))
  (bind _returnvalue_3 (Ability|GetAvatarActorfromActorInfo))
  (Variables|Default|SetHasHitTarget false)
  (bind _returnvalue_4 (Class|CombatInterface|GetAttackMontages(Message) (Ability|GetAvatarActorfromActorInfo)))
  (Variables|Default|SetCurrentTaggedMontage (.OutItem (Utilities|Array|Random _returnvalue_4)))
  (Variables|Default|SetImpact%20Sound (.ImpactSound (Utilities|Struct|BreakTaggedMontage (Variables|Default|GetCurrentTaggedMontage))))
  (Variables|Default|SetMontage%20Tag (.MontageTag (Utilities|Struct|BreakTaggedMontage (Variables|Default|GetCurrentTaggedMontage))))
  (Variables|Default|SetSocket%20Tag (.SocketTag (Utilities|Struct|BreakTaggedMontage (Variables|Default|GetCurrentTaggedMontage))))
  (|PlayMontageandWaitProxy "None" (.Montage (Utilities|Struct|BreakTaggedMontage (Variables|Default|GetCurrentTaggedMontage))) 1.0 "None" false 1.0 0.0 false
    (:then
      (bind _returnvalue_5 (Class|EnemyInterface|GetCombatTarget(Message) _returnvalue))
      (Class|CombatInterface|SetMotionWarpTarget(Message) _returnvalue (Transformation|GetActorLocation _returnvalue_5))
      (Ability|Tasks|WaitGameplayEvent (Variables|Default|GetMontage%20Tag) 0
        (:EventReceived
          (bind _returnvalue_6 (Class|CombatInterface|GetCombatSocketLocation(Message) (Ability|GetAvatarActorfromActorInfo) (Variables|Default|GetSocket%20Tag)))
          (Variables|Default|SetCombatSocketLocation _returnvalue_6)
          (if (Variables|Default|GetDrawDebug)
            (Rendering|Debug|DrawDebugSphere (Variables|Default|GetCombatSocketLocation) 6e+01 12 "(R=1.000000,G=0.083333,B=0.083333,A=1.000000)" 0.5))
          (bind _outliveplayers (Class|AuraAbilitySystemLibrary|GetLivePlayersWithinRadius _returnvalue_3 (Utilities|Array|MakeArray _returnvalue_3) 6e+01 (Variables|Default|GetCombatSocketLocation)))
          (for _array_element _outliveplayers
            (if (Class|AuraAbilitySystemLibrary|IsEnemyTeam _array_element (Ability|GetAvatarActorfromActorInfo))
              (Class|AuraDamageGameplayAbility|CauseDamage _array_element)
              (Variables|Default|SetHasHitTarget true)))
          (if (Variables|Default|GetHasHitTarget)
            (bind _returnvalue_7 (Class|EnemyInterface|GetCombatTarget(Message) _returnvalue_2))
            (Class|GameplayAbility|ExecuteGameplayCuewithParams "(TagName=\"GameplayCue.MeleeImpact\")" (Ability|GameplayCue|MakeGameplayCueParameters :AggregatedSourceTags (GameplayTags|MakeGameplayTagContainerfromTag (Variables|Default|GetMontage%20Tag)) :Location (Variables|Default|GetCombatSocketLocation) :EffectCauser _returnvalue_2 :SourceObject _returnvalue_7)) ; TODO: Get hit result and execute for each target hit
          ))))
    (:OnCompleted
      (Ability|EndAbility :!label _label))
    (:OnInterrupted
      (goto _label))
    (:OnCancelled
      (goto _label))))
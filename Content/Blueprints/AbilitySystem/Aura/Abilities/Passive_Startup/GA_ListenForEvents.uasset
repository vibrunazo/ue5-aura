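; Passive startup gameplay ability for Aura that listens for gameplay events under the Attributes tag and turns them into attribute effects on itself.
; On activation it waits for events matching that tag or its child tags.
; Each event's tag and magnitude become a SetByCaller value on a spec from MakeSpecFromEffectClass, which is applied to the owner's ability system component.
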(event Ability|EventActivateAbility
  (Development|PrintString "Listening for events")
  (bind _payload (Ability|Tasks|WaitGameplayEvent "(TagName=\"Attributes\")" 0 false false)
    (:EventReceived
      (bind _returnvalue (Ability|GameplayEffect|AssignTagSetbyCallerMagnitude (|MakeSpecFromEffectClass) (.EventTag (Utilities|Struct|BreakGameplayEventData _payload)) (.EventMagnitude (Utilities|Struct|BreakGameplayEventData _payload))))
      (GameplayEffects|ApplyGameplayEffectSpecToSelf (Ability|GetAbilitySystemComponentfromActorInfo) _returnvalue))))
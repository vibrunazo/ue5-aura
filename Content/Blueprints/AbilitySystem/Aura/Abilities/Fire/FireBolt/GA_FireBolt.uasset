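; Fire bolt Gameplay Ability that casts a projectile toward the point under the mouse.
; On activation it commits, requests cursor target data, and ends if none is valid by the next tick.
; Valid data plays the cast montage and feeds the impact point to motion warping.
; A weapon-socket gameplay event triggers the projectile, and the montage finishing or being interrupted ends the ability.
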(event Ability|EventActivateAbility
  (Ability|CommitAbility)
  (Variables|Default|SetIsTargetDataValid false)
  (bind _datahandle (|TargetDataUnderMouse)
    (:then
      (Utilities|FlowControl|DelayUntilNextTick)
      (if (not (Variables|Default|GetIsTargetDataValid))
        (Ability|EndAbility)))
    (:ValidData
      (Variables|Default|SetIsTargetDataValid true)
      (|PlayMontageandWaitProxy "None" "/Game/Assets/Characters/Aura/Animations/Abilities/AM_CastFireBolt.AM_CastFireBolt" 1.0 "None" false 1.0 0.0 false
        (:then
          (Class|CombatInterface|SetMotionWarpTarget(Message) (Ability|GetAvatarActorfromActorInfo) (.ImpactPoint (Collision|BreakHitResult (Ability|TargetData|GetHitResultfromTargetData _datahandle))))
          (Ability|Tasks|WaitGameplayEvent "(TagName=\"CombatSocket.Weapon\")" 0
            (:EventReceived
              (Class|AuraProjectileSpell|CastProjectile (.ImpactPoint (Collision|BreakHitResult (Ability|TargetData|GetHitResultfromTargetData _datahandle))) "(TagName=\"CombatSocket.Weapon\")" 0.0 "0, 0, 0"))))
        (:OnCompleted
          (Ability|EndAbility :!label _label))
        (:OnBlendOut
          (goto _label))
        (:OnInterrupted
          (goto _label))
        (:OnCancelled
          (goto _label))))))

(event Ability|EventOnEndAbility
  (params (bWasCancelled :type Boolean)))